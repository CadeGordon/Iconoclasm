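; Blood splatter preset actor that fires a Niagara burst of droplets on BeginPlay and leaves bloodstains from them.
; Exposed settings drive the burst's gravity, speed, size, count and color, and the actor registers itself as the Niagara export callback.
; For each particle received in ParticleData, it spawns a BP_Bloodstain_Main oriented by velocity, with randomized scale adjusted by particle size, random yaw, a random tinted material and a set lifetime.
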(event `self.ReceiveBeginPlay`
  (`self.SpawnDrops`))

(event `SpawnDrops`
  (bind _dropletstyle_niagara (`self.DropletStyle_Niagara`))
  (bind _particle_maxdistance (`self.Particle_MaxDistance`))
  (bind _dropletstyle_niagara_2 (`self.DropletStyle_Niagara`))
  ;[0 0.02129 1] SPAWN DROPs
  (`NiagaraComponent.SetAsset` _dropletstyle_niagara_2 (`self.Burst_Style`))
  (`NiagaraComponent.SetVariableFloat` _dropletstyle_niagara_2 "Gravity_Scale" (`self.Gravity_Scale`))
  (`NiagaraComponent.SetVariableFloat` _dropletstyle_niagara_2 "SpeetMultiplier_Max" _particle_maxdistance)
  (`NiagaraComponent.SetVariableFloat` _dropletstyle_niagara_2 "Dist" (+ (`self.Particle_LifeTime_Multiplier`) _particle_maxdistance))
  (`NiagaraComponent.SetVariableFloat` _dropletstyle_niagara_2 "SpeedMultiplier" (`self.Particle_Min_Distance`))
  (`NiagaraComponent.SetVariableFloat` _dropletstyle_niagara_2 "Particle_Sizew" (`self.Particle_Size`))
  (`NiagaraComponent.SetVariableInt` _dropletstyle_niagara_2 "Spawn_Rate" (`self.Max_Drops`))
  (`NiagaraComponent.SetNiagaraVariableObject` _dropletstyle_niagara "User.BP_CallBack" self)
  (`NiagaraComponent.SetVariableLinearColor` _dropletstyle_niagara "Color" (`self.Color`))
  (`ActorComponent.Activate` (`self.DropletStyle_Niagara`) true))

(event `self.ReceiveParticleData`
  (params (Data :type "Array of BasicParticleData Structure (by ref)") (NiagaraSystem :type "NiagaraSystem Object Reference"))
  (bind _splat_materials (`self.Splat_Materials`))
  ;[1 0.2708 0.7189] SPLAT SPAWN
  (bind (_position _size _velocity) (break `BasicParticleData` (stale _array_element)))
  (bind _returnvalue (`|SpawnActorFromClass` "/Game/sA_BloodSplatter_System/Blueprints/BP_Bloodstain_Main.BP_Bloodstain_Main_C" (`KismetMathLibrary.MakeTransform` _position (`KismetMathLibrary.MakeRotFromZ` _velocity) (`KismetMathLibrary.Conv_DoubleToVector` (/ (`KismetMathLibrary.RandomFloatInRange` (`self.SplatSize_Min`) (`self.SplatSize_Max`)) (`KismetMathLibrary.FClamp` (/ (`KismetMathLibrary.FClamp` _size 100.0 1000.0) 100.0) 1.0 (* (`KismetMathLibrary.FClamp` (`self.SplatSize_Max`) 1.0 999999.0) 10.0))))) "Undefined" "OverrideRootScale" null null))
  (bind _plane (`/Game/sA_BloodSplatter_System/Blueprints/BP_Bloodstain_Main.Plane` _returnvalue))
  (bind (_relativerotation_roll _relativerotation_pitch) (`KismetMathLibrary.BreakRotator` (`SceneComponent.RelativeRotation` _plane)))
  (`SceneComponent.K2_SetRelativeRotation` _plane (`KismetMathLibrary.MakeRotator` _relativerotation_roll _relativerotation_pitch (`KismetMathLibrary.RandomFloatInRange` 0.0 50.0)) false false)
  ;;[1 0 0.3694] Random Material Section
  (bind _returnvalue_2 (`KismetMaterialLibrary.CreateDynamicMaterialInstance` (`|GetArrayItem` _splat_materials (`KismetMathLibrary.RandomIntegerInRange` 0 (- (`KismetArrayLibrary.Array_Length` _splat_materials) 1)))))
  (`MaterialInstanceDynamic.SetVectorParameterValue` _returnvalue_2 "Color" (`self.Color`))
  (`PrimitiveComponent.SetMaterial` _plane 0 _returnvalue_2)
  (set `/Game/sA_BloodSplatter_System/Blueprints/BP_Bloodstain_Main.Lifetime` (`self.Splat_Duration`) _returnvalue)
  (for _array_element Data
    _))

(fn `UserConstructionScript`)