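; BP_OpenShop is an interactable actor that opens the shop home screen for the player.
; Its InteractBOx overlap adds the WBP_Interact widget when the player character enters and removes it on exit.
; The Interact event, whose caller is outside this graph, creates WBP_ShopHome, switches input to UI-only and shows the mouse cursor.
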(event `self.Interact`
  (bind _returnvalue (`GameplayStatics.GetPlayerController` 0))
  (bind _returnvalue_2 (`|CreateWidget` "/Game/UI/WBP_ShopHome.WBP_ShopHome_C"))
  (`UserWidget.AddToViewport` _returnvalue_2 0)
  (`WidgetBlueprintLibrary.SetInputMode_UIOnlyEx` _returnvalue null)
  (set `PlayerController.bShowMouseCursor` true _returnvalue))

(event `self.InteractBOx.OnComponentBeginOverlap`
  (params (OverlappedComponent :type "PrimitiveComponent Object Reference") (OtherActor :type "Actor Object Reference") (OtherComp :type "PrimitiveComponent Object Reference") (OtherBodyIndex :type Integer) (bFromSweep :type Boolean) (SweepResult :type "HitResult Structure (by ref)"))
  (if (== OtherActor (`GameplayStatics.GetPlayerCharacter` 0))
    (bind _returnvalue (`|CreateWidget` "/Game/UI/WBP_Interact.WBP_Interact_C"))
    (`UserWidget.AddToViewport` _returnvalue 0)))

(event `self.InteractBOx.OnComponentEndOverlap`
  (params (OverlappedComponent :type "PrimitiveComponent Object Reference") (OtherActor :type "Actor Object Reference") (OtherComp :type "PrimitiveComponent Object Reference") (OtherBodyIndex :type Integer))
  (if (== (`GameplayStatics.GetPlayerCharacter` 0) OtherActor)
    (`Widget.RemoveFromParent` (stale `self.InteractBOx.OnComponentBeginOverlap` _returnvalue))))

(fn `UserConstructionScript`)